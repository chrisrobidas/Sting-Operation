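; BP_Door is a stone door actor that opens once by sinking downward and then removes itself.
; RemoveDoor, guarded by IsOpened, plays the stone door sound and starts the MoveDoor timeline.
; Each update lerps from the actor's current location toward a point below it, so the descent accumulates rather than following fixed endpoints.
; When the timeline finishes, the actor is destroyed after a short delay.
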(event Custom|RemoveDoor
  (bind _returnvalue (Transformation|GetActorLocation))
  (if (not (Variables|Default|GetIsOpened))
    (Variables|Default|SetIsOpened true)
    (Audio|PlaySoundatLocation "/Game/LudmDare56/Assets/Audio/stone_door.stone_door" (Transformation|GetWorldLocation (Variables|Default|GetStaticMesh)) "0, 0, 0" 1.0 1.0 0.0 0 0 0 0)
    (bind _alpha (Timeline|MoveDoor Play)
      (:Update
        (Transformation|SetActorLocation (Math|Vector|Lerp(Vector) _returnvalue (- _returnvalue "0.000000,0.000000,50.000000") _alpha) false false))
      (:Finished
        (Utilities|FlowControl|Delay 2.0)
        (Actor|DestroyActor)))))

(event EventBeginPlay)

(event Collision|EventActorBeginOverlap
  (params (OtherActor :type Actor%20Object%20Reference)))

(event EventTick
  (params (DeltaSeconds :type Float%20%28single-precision%29)))

(fn ConstructionScript)