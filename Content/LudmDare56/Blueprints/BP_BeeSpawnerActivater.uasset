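; Trigger-box actor that activates a set of bee spawners and can open a door once the bees are gone.
; On BeginPlay it registers itself with each listed spawner, and the first player overlap makes them all spawn bees.
; Once active with OpenDoor set, a delayed Tick check finds no enemies left in the box, then removes the linked door.
; With FinishGame set, it only prints a placeholder message instead.
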(event OnComponentBeginOverlap(Box)
  (params (OverlappedComponent :type Primitive%20Component%20Object%20Reference) (OtherActor :type Actor%20Object%20Reference) (OtherComp :type Primitive%20Component%20Object%20Reference) (OtherBodyIndex :type Integer) (bFromSweep :type Boolean) (SweepResult :type Hit%20Result%20Structure%20%28by%20ref%29))
  (Utilities|Casting|CastToBP_FirstPersonCharacter OtherActor)
  (if (not (Variables|Default|GetbBeesActivated))
    (Variables|Default|SetbBeesActivated true)
    (for _array_element (Variables|Default|GetBeeSpawnersList)
      (Default|SpawnBees _array_element))))

(event EventBeginPlay
  (for _array_element (Variables|Default|GetBeeSpawnersList)
    (Variables|/Game/LudmDare56/Blueprints/BP_BeeSpawner.BP_BeeSpawner_C|SetSpawnerActivaterRef _array_element self)))

(event Collision|EventActorBeginOverlap
  (params (OtherActor :type Actor%20Object%20Reference)))

(event EventTick
  (params (DeltaSeconds :type Float%20%28single-precision%29))
  (bind _doorref (Variables|Default|GetDoorRef))
  (if (and (Variables|Default|GetbBeesActivated) (Variables|Default|GetbOpenDoor))
    (Utilities|FlowControl|Delay 3.0)
    (bind _output_get (Variables|Default|SetOverlappingBees (Collision|GetOverlappingActors (Variables|Default|GetBox) "/Game/LudmDare56/Blueprints/EnemyAI/BP_EnemyAICharacter.BP_EnemyAICharacter_C" :!class /Script/Engine.PrimitiveComponent)))
    (if (Utilities|Array|IsEmpty _output_get)
      (if (Variables|Default|GetbFinishGame)
        (Development|PrintString "Hello")
        (elif (Utilities|IsValid _doorref)
          (Default|RemoveDoor _doorref))))))

(fn ConstructionScript)