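; BP_Instance, apparently the game instance, owns the game's save data, loading a BP_Save from a slot on Init or creating one if none exists.
; Loads broadcast a save-loaded event, plus a player-loaded event when an existing save is loaded with Load set.
; SavePlayer stores player data and writes it synchronously or asynchronously.
; Loading repeats the existence check, so only its async path runs.
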(event EventInit
  (CallFunction|LoadGameData false))

(event EventSaveGameData
  (params (Async :type Boolean))
  ;[1 1 1] Save Game
  (if Async
    (|AsyncSaveGametoSlot (Variables|Default|GetSaveGame) (Variables|Default|GetSlotName))
    (else
      (SaveGame|SaveGametoSlot (Variables|Default|GetSaveGame) (Variables|Default|GetSlotName)))))

(event EventLoadGameData
  (params (Async :type Boolean))
  ;[1 1 1] Load Game
  (bind _returnvalue (SaveGame|DoesSaveGameExist (Variables|Default|GetSlotName)))
  (if _returnvalue
    (if _returnvalue
      (bind _savegame (|AsyncLoadGamefromSlot (Variables|Default|GetSlotName))
        (:Completed
          (bind _asbp_save (Utilities|Casting|CastToBP_Save _savegame))
          (bind _output_get (Variables|Default|SetSaveGame _asbp_save))
          (Default|CallOnSaveLoaded _output_get)
          (if (Variables|Default|GetbLoad)
            (Default|CallOnPlayerLoaded _output_get))))
      (else
        (bind _returnvalue_2 (SaveGame|LoadGamefromSlot (Variables|Default|GetSlotName)))
        (bind _asbp_save_2 (Utilities|Casting|CastToBP_Save _returnvalue_2))
        (bind _output_get_2 (Variables|Default|SetSaveGame _asbp_save_2))
        (Default|CallOnSaveLoaded _output_get_2)
        (if (Variables|Default|GetbLoad)
          (Default|CallOnPlayerLoaded _output_get_2))))
    (else
      (CallFunction|CreateNewGame)
      (Default|CallOnSaveLoaded (Variables|Default|GetSaveGame)))))

(event EventSavePlayer
  (params (PlayerSave :type S%20Player%20Data%20Structure) (Async :type Boolean))
  (if (and (CallFunction|HasSave) (Utilities|IsValid (Variables|Default|GetSaveGame)))
    _
    (else
      (CallFunction|CreateNewGame)))
  (Variables|/Game/LudmDare56/Blueprints/SaveGame/BP_Save.BP_Save_C|SetPlayerData (Variables|Default|GetSaveGame) PlayerSave)
  (CallFunction|SaveGameData Async))

(fn CreateNewGame
  (bind _returnvalue (SaveGame|CreateSaveGameObject "/Game/LudmDare56/Blueprints/SaveGame/BP_Save.BP_Save_C"))
  (Variables|Default|SetSaveGame _returnvalue))

(fn HasSave
  (bind _returnvalue (SaveGame|DoesSaveGameExist (Variables|Default|GetSlotName)))
  (return _returnvalue))

(fn GetSave
  (bind _savegame (Variables|Default|GetSaveGame))
  (if (and (Utilities|IsValid _savegame) (CallFunction|HasSave))
    _
    (else
      (CallFunction|CreateNewGame)))
  (return _savegame))

(fn GetGameData
  (return (Variables|Default|GetSaveGame)))