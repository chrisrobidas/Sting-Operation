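; BP_Checkpoint is a numbered checkpoint actor that saves player progress when the first-person character overlaps its sphere.
; It only saves when its CheckpointNumber exceeds the one in the game instance's save, so progress never moves backward.
; It takes the character's save data, substitutes its own checkpoint number, and passes it to the game instance's SavePlayer message.
; The game-loaded delegate binding is disconnected and never runs.
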(event OnComponentBeginOverlap(Sphere)
  (params (OverlappedComponent :type Primitive%20Component%20Object%20Reference) (OtherActor :type Actor%20Object%20Reference) (OtherComp :type Primitive%20Component%20Object%20Reference) (OtherBodyIndex :type Integer) (bFromSweep :type Boolean) (SweepResult :type Hit%20Result%20Structure%20%28by%20ref%29))
  (bind _asbp_instance (Utilities|Casting|CastToBP_Instance (Game|GetGameInstance)))
  (if (> (Variables|Default|GetCheckpointNumber) (.CheckpointNumber (Utilities|Struct|BreakS_PlayerData (Variables|/Game/LudmDare56/Blueprints/SaveGame/BP_Save.BP_Save_C|GetPlayerData (Default|GetSave _asbp_instance)))))
    (bind _asbp_first_person_character (Utilities|Casting|CastToBP_FirstPersonCharacter OtherActor))
    (bind _player_save (Default|GetPlayerSave _asbp_first_person_character))
    (Class|BPISaveGame|SavePlayer(Message) (Game|GetGameInstance) (Utilities|Struct|MakeS_PlayerData (.PlayerHealth (Utilities|Struct|BreakS_PlayerData _player_save)) (.PlayerAmmo (Utilities|Struct|BreakS_PlayerData _player_save)) (.PlayerHoney (Utilities|Struct|BreakS_PlayerData _player_save)) (.PlayerPosition (Utilities|Struct|BreakS_PlayerData _player_save)) (.PlayerCamPosition (Utilities|Struct|BreakS_PlayerData _player_save)) (.LevelName (Utilities|Struct|BreakS_PlayerData _player_save)) (Variables|Default|GetCheckpointNumber) (.HoldingGun (Utilities|Struct|BreakS_PlayerData _player_save))) false)))

(event Custom|OnGameLoaded_Event
  (params (SaveGame :type BP%20Save%20Object%20Reference))
  (Variables|Default|SetSave%20Game SaveGame))

(event EventBeginPlay)

(event Collision|EventActorBeginOverlap
  (params (OtherActor :type Actor%20Object%20Reference)))

(event EventTick
  (params (DeltaSeconds :type Float%20%28single-precision%29)))

(fn ConstructionScript)