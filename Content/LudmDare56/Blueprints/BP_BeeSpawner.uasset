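; BP_BeeSpawner is a spawner actor that releases a set number of bee enemies (BP_EnemyAICharacter) at its own transform.
; Shortly after BeginPlay it adds its bee count to the kill target on its linked SpawnerActivaterRef.
; The SpawnBees event, not triggered within this Blueprint, loops with a delay between spawns until the count runs out, then destroys the spawner.
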(event Custom|SpawnBees
  (if (> (Variables|Default|GetNbBeesToSpawn) 0) :!label _label
    (Game|SpawnActorfromClass "/Game/LudmDare56/Blueprints/EnemyAI/BP_EnemyAICharacter.BP_EnemyAICharacter_C" (Transformation|GetActorTransform) "Undefined" "MultiplyWithRoot" 0 0)
    (Variables|Default|SetNbBeesToSpawn (- (Variables|Default|GetNbBeesToSpawn) 1))
    (Utilities|FlowControl|Delay (Math|Conversions|ToFloat(Integer) (Variables|Default|GetTimerBetweenBeeSpawns)))
    (goto _label)
    (else
      (Utilities|FlowControl|Delay 0.2)
      (Actor|DestroyActor self))))

(event EventBeginPlay
  (bind _spawneractivaterref (Variables|Default|GetSpawnerActivaterRef))
  (Utilities|FlowControl|Delay 0.2)
  (if (Utilities|IsValid _spawneractivaterref)
    (Variables|/Game/LudmDare56/Blueprints/BP_BeeSpawnerActivater.BP_BeeSpawnerActivater_C|SetNbBeesToKill _spawneractivaterref (+ (Variables|/Game/LudmDare56/Blueprints/BP_BeeSpawnerActivater.BP_BeeSpawnerActivater_C|GetNbBeesToKill _spawneractivaterref) (Variables|Default|GetNbBeesToSpawn)))))

(event Collision|EventActorBeginOverlap
  (params (OtherActor :type Actor%20Object%20Reference)))

(event EventTick
  (params (DeltaSeconds :type Float%20%28single-precision%29)))

(fn ConstructionScript)